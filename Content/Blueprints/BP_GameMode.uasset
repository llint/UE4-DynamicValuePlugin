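; Game mode that exercises a DynamicValue type system with mixed-type arrays, parsed JSON and per-team actor sets.
; BeginPlay runs Initialize to build the team map, an embedded network-style JSON config and a sample array.
; Manipulate, not called within this graph, prints both through type-dispatched dump functions and spawns tagged BP_Cube columns for TeamA and TeamB.
; ActorClicked uses the team tag to remove a cube from its set and destroy it.
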(event Custom|ActorClicked
  (params (Actor :type Actor%20Object%20Reference))
  (if (Actor|ActorHasTag Actor "TeamA")
    (CallFunction|DestroyTeamActor Actor "TeamA")
    (elif (Actor|ActorHasTag Actor "TeamB")
      (CallFunction|DestroyTeamActor Actor "TeamB"))))

(event EventBeginPlay
  (CallFunction|Initialize))

(fn ConstructionScript)

(fn Initialize
  (bind _output_get (Variables|Default|SetTeamPlayers (Class|StringtoDynamicValueMap|MakeStringtoDynamicValueMap)))
  (bind _returnvalue (Class|StringtoDynamicValueMap|Add _output_get "TeamA" (Class|DynamicValueLibrary|MakeDynamicValueActorSet)))
  (Class|StringtoDynamicValueMap|Add _returnvalue "TeamB" (Class|DynamicValueLibrary|MakeDynamicValueActorSet))
  (Variables|Default|SetGameConfig (Class|DynamicStructLibrary|ParseJsonString "{
    \"FactoryDefault\" :
    {
        \"Zones\" :
        [{
            \"Name\" : \"Loopback\",
            \"Interface\" : \"lo\",
            \"IP\" : \"127.0.0.1\"
        }]
    },
    \"UserConfig\" :
    {
        \"Interfaces\" : [\"eth0\", \"lo\", \"eth1\"],
        \"Zones\" :
        [{
            \"Name\" : \"Internal\",
            \"Interface\" : \"eth0\",
            \"IP\" : \"192.168.1.1/24\",
            \"EnableRouting\" : true,
            \"PortMapping\" :
            [{
                \"SrcPort\" : 8080,
                \"DestIP\" : \"192.168.1.10\",
                \"DestPort\" : 80
            }]
        },
        {
            \"Name\" : \"External\",
            \"Interface\" : \"eth1\",
            \"UseDhcp\"   : true
        }]
    }
}"))
  (Utilities|Array|Add (Variables|Default|GetHeterogeneousArray) (Class|DynamicValueLibrary|MakeDynamicValueBoolean true))
  (Utilities|Array|Add (Variables|Default|GetHeterogeneousArray) (Class|DynamicValueLibrary|MakeDynamicValueInteger 123))
  (Utilities|Array|Add (Variables|Default|GetHeterogeneousArray) (Class|DynamicValueLibrary|MakeDynamicValueFloat 0.123))
  (Utilities|Array|Add (Variables|Default|GetHeterogeneousArray) (Class|DynamicValueLibrary|MakeDynamicValueString "Hello"))
  (Utilities|Array|Add (Variables|Default|GetHeterogeneousArray) (Class|DynamicValueLibrary|MakeDynamicValueVector "0, 0, 0"))
  (Utilities|Array|Add (Variables|Default|GetHeterogeneousArray) (Class|DynamicValueLibrary|MakeDynamicValueStruct))
  (Utilities|Array|Add (Variables|Default|GetHeterogeneousArray) (Class|DynamicValueLibrary|MakeDynamicValueArray))
  (return))

(fn Manipulate
  (for _array_element (Variables|Default|GetHeterogeneousArray)
    (CallFunction|DumpDynamicValue _array_element))
  (CallFunction|DumpGameConfig)
  (CallFunction|CreateTeamPlayers "TeamA" "0.000000, 0, 0")
  (CallFunction|CreateTeamPlayers "TeamB" "200.000000,0.000000, 0"))

(fn DumpDynamicValue
  (params (Value :type Dynamic%20Value%20Object%20Reference))
  (bind _output_get (LocalVariables|SetLocalValue Value))
  (switch Utilities|FlowControl|Switch|SwitchonEDynamicValueType (Class|DynamicValue|GetType _output_get)
    (:None
      (Development|PrintString "DynamicValue: None" true true "(R=0.000000,G=0.660000,B=1.000000,A=1.000000)" 1e+01))
    (:Boolean
      (CallFunction|DumpDynamicValueasBoolean (LocalVariables|GetLocalValue)))
    (:Integer
      (CallFunction|DumpDynamicValueasInteger (LocalVariables|GetLocalValue)))
    (:Float
      (CallFunction|DumpDynamicValueasFloat (LocalVariables|GetLocalValue)))
    (:String
      (CallFunction|DumpDynamicValueasString (LocalVariables|GetLocalValue)))
    (:Vector
      (CallFunction|DumpDynamicValueasVector (LocalVariables|GetLocalValue)))
    (:Array
      (CallFunction|DumpDynamicValueasArray (LocalVariables|GetLocalValue)))
    (:Struct
      (CallFunction|DumpDynamicValueasStruct (LocalVariables|GetLocalValue)))))

(fn DumpDynamicValueasBoolean
  (params (Value :type Dynamic%20Value%20Object%20Reference))
  (bind _asdynamic_value_boolean (Utilities|Casting|CastToDynamicValueBoolean Value))
  (Development|PrintString (Utilities|String|Append "DynamicValueBoolean: " (Utilities|String|ToString(Boolean) (Variables|/Script/DynamicValuePlugin.DynamicValueBoolean|GetValue _asdynamic_value_boolean)))))

(fn DumpDynamicValueasInteger
  (params (Value :type Dynamic%20Value%20Object%20Reference))
  (bind _asdynamic_value_integer (Utilities|Casting|CastToDynamicValueInteger Value))
  (Development|PrintString (Utilities|String|Append "DynamicValueInteger: " (Utilities|String|ToString(Integer) (Variables|/Script/DynamicValuePlugin.DynamicValueInteger|GetValue _asdynamic_value_integer)))))

(fn DumpDynamicValueasFloat
  (params (Value :type Dynamic%20Value%20Object%20Reference))
  (bind _asdynamic_value_float (Utilities|Casting|CastToDynamicValueFloat Value))
  (Development|PrintString (Utilities|String|Append "DynamicValueFloat: " (Utilities|String|ToString(Float) (Variables|/Script/DynamicValuePlugin.DynamicValueFloat|GetValue _asdynamic_value_float)))))

(fn DumpDynamicValueasString
  (params (Value :type Dynamic%20Value%20Object%20Reference))
  (bind _asdynamic_value_string (Utilities|Casting|CastToDynamicValueString Value))
  (Development|PrintString (Utilities|String|Append "DynamicValueString: " (Variables|/Script/DynamicValuePlugin.DynamicValueString|GetValue _asdynamic_value_string))))

(fn DumpDynamicValueasVector
  (params (Value :type Dynamic%20Value%20Object%20Reference))
  (bind _asdynamic_value_vector (Utilities|Casting|CastToDynamicValueVector Value))
  (Development|PrintString (Utilities|String|Append "DynamicValueVector: " (Utilities|String|ToString(Vector) (Variables|/Script/DynamicValuePlugin.DynamicValueVector|GetValue _asdynamic_value_vector)))))

(fn DumpDynamicValueasArray
  (params (Value :type Dynamic%20Value%20Object%20Reference))
  (bind _asdynamic_value_array (Utilities|Casting|CastToDynamicValueArray Value))
  (for _array_element (Variables|/Script/DynamicValuePlugin.DynamicValueArray|GetValue _asdynamic_value_array)
    (CallFunction|DumpDynamicValue _array_element)))

(fn DumpDynamicValueasStruct
  (params (Value :type Dynamic%20Value%20Object%20Reference))
  ;[1 1 1] It is not possible to iterate through the fields just for the sake of printing ...
  (bind _asdynamic_value_struct (Utilities|Casting|CastToDynamicValueStruct Value))
  (Development|PrintString (Utilities|GetDisplayName (Variables|/Script/DynamicValuePlugin.DynamicValueStruct|GetValue _asdynamic_value_struct))))

(fn DumpGameConfig
  (Utilities|FlowControl|Sequence
    (:then_0
      (bind _returnvalue (Class|DynamicStruct|GetField (Variables|Default|GetGameConfig) "FactoryDefault"))
      (bind _asdynamic_value_struct (Utilities|Casting|CastToDynamicValueStruct _returnvalue))
      (bind _returnvalue_2 (Class|DynamicStruct|GetField (Variables|/Script/DynamicValuePlugin.DynamicValueStruct|GetValue _asdynamic_value_struct) "Zones"))
      (CallFunction|DumpZones _returnvalue_2))
    (:then_1
      (bind _returnvalue_3 (Class|DynamicStruct|GetField (Variables|Default|GetGameConfig) "UserConfig"))
      (bind _asdynamic_value_struct_2 (Utilities|Casting|CastToDynamicValueStruct _returnvalue_3))
      (bind _returnvalue_4 (Class|DynamicStruct|GetField (Variables|/Script/DynamicValuePlugin.DynamicValueStruct|GetValue _asdynamic_value_struct_2) "Interfaces"))
      (CallFunction|DumpDynamicValueasArray _returnvalue_4)
      (bind _returnvalue_5 (Class|DynamicStruct|GetField (Variables|/Script/DynamicValuePlugin.DynamicValueStruct|GetValue _asdynamic_value_struct_2) "Zones"))
      (CallFunction|DumpZones _returnvalue_5))))

(fn DumpZones
  (params (Zones :type Dynamic%20Value%20Object%20Reference))
  (bind _asdynamic_value_array (Utilities|Casting|CastToDynamicValueArray Zones))
  (for _array_element (Variables|/Script/DynamicValuePlugin.DynamicValueArray|GetValue _asdynamic_value_array)
    (bind _asdynamic_value_struct (Utilities|Casting|CastToDynamicValueStruct _array_element))
    (bind _returnvalue (Class|DynamicStruct|GetField (Variables|/Script/DynamicValuePlugin.DynamicValueStruct|GetValue _asdynamic_value_struct) "Name"))
    (CallFunction|DumpDynamicValueasString _returnvalue)
    (bind _returnvalue_2 (Class|DynamicStruct|GetField (Variables|/Script/DynamicValuePlugin.DynamicValueStruct|GetValue _asdynamic_value_struct) "Interface"))
    (CallFunction|DumpDynamicValueasString _returnvalue_2)
    (bind _returnvalue_3 (Class|DynamicStruct|GetField (Variables|/Script/DynamicValuePlugin.DynamicValueStruct|GetValue _asdynamic_value_struct) "IP"))
    (CallFunction|DumpDynamicValueasString _returnvalue_3)
    (bind _returnvalue_4 (Class|DynamicStruct|GetField (Variables|/Script/DynamicValuePlugin.DynamicValueStruct|GetValue _asdynamic_value_struct) "EnableRouting"))
    (CallFunction|DumpDynamicValueasBoolean _returnvalue_4)
    (bind _returnvalue_5 (Class|DynamicStruct|GetField (Variables|/Script/DynamicValuePlugin.DynamicValueStruct|GetValue _asdynamic_value_struct) "UseDhcp"))
    (CallFunction|DumpDynamicValueasBoolean _returnvalue_5)
    (bind _returnvalue_6 (Class|DynamicStruct|GetField (Variables|/Script/DynamicValuePlugin.DynamicValueStruct|GetValue _asdynamic_value_struct) "PortMapping"))
    (bind _asdynamic_value_array_2 (Utilities|Casting|CastToDynamicValueArray _returnvalue_6))
    (for _array_element_2 (Variables|/Script/DynamicValuePlugin.DynamicValueArray|GetValue _asdynamic_value_array_2)
      (bind _asdynamic_value_struct_2 (Utilities|Casting|CastToDynamicValueStruct _array_element_2))
      (bind _returnvalue_7 (Class|DynamicStruct|GetField (Variables|/Script/DynamicValuePlugin.DynamicValueStruct|GetValue _asdynamic_value_struct_2) "SrcPort"))
      (CallFunction|DumpDynamicValueasFloat _returnvalue_7)
      (bind _returnvalue_8 (Class|DynamicStruct|GetField (Variables|/Script/DynamicValuePlugin.DynamicValueStruct|GetValue _asdynamic_value_struct_2) "DestIP"))
      (CallFunction|DumpDynamicValueasString _returnvalue_8)
      (bind _returnvalue_9 (Class|DynamicStruct|GetField (Variables|/Script/DynamicValuePlugin.DynamicValueStruct|GetValue _asdynamic_value_struct_2) "DestPort"))
      (CallFunction|DumpDynamicValueasFloat _returnvalue_9))))

(fn CreateTeamPlayers
  (params (Team :type String) (Start :type Vector))
  (bind (_x _y _z) (Math|Vector|BreakVector Start))
  (bind _asdynamic_value_actor_set (Utilities|Casting|CastToDynamicValueActorSet (Class|StringtoDynamicValueMap|GetValue (Variables|Default|GetTeamPlayers) Team)))
  (for _index (range 0 9)
    (bind _returnvalue (Game|SpawnActorfromClass "/Game/Blueprints/BP_Cube.BP_Cube_C" (Math|Transform|MakeTransform (Math|Vector|MakeVector _x _y (+ _z (* _index 2e+02)))) "AdjustIfPossibleButAlwaysSpawn" 0 0))
    (Variables|/Script/Engine.Actor|SetTags _returnvalue (Utilities|Array|MakeArray (Utilities|String|StringToName Team)))
    (Class|ActorSet|Add (Variables|/Script/DynamicValuePlugin.DynamicValueActorSet|GetValue _asdynamic_value_actor_set) _returnvalue)))

(fn DestroyTeamActor
  (params (Actor :type Actor%20Object%20Reference) (Team :type Name))
  (bind _asdynamic_value_actor_set (Utilities|Casting|CastToDynamicValueActorSet (Class|StringtoDynamicValueMap|GetValue (Variables|Default|GetTeamPlayers) (Utilities|String|ToString(Name) Team))))
  (if (Class|ActorSet|Contains (Variables|/Script/DynamicValuePlugin.DynamicValueActorSet|GetValue _asdynamic_value_actor_set) Actor)
    (bind _returnvalue (Class|ActorSet|Remove (Variables|/Script/DynamicValuePlugin.DynamicValueActorSet|GetValue _asdynamic_value_actor_set) Actor))
    (if _returnvalue
      (Actor|DestroyActor Actor))))